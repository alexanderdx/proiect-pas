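; Hunter AI animal, using lion animations, that chases prey and can be killed.
; When a PreyAI capsule enters the sensing sphere, it writes that prey to the blackboard, switches to chasing speed and resets the player-target timer.
; HunterDeath runs once, playing the death montage, removing the sensing sphere and capsule, and stopping controller movement.
; IsInterestedInPawn accepts only FpsPasCharacter pawns.
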(event OnComponentBeginOverlap(SensingSphere)
  (params (OverlappedComponent :type Primitive%20Component%20Object%20Reference) (OtherActor :type Actor%20Object%20Reference) (OtherComp :type Primitive%20Component%20Object%20Reference) (OtherBodyIndex :type Integer) (bFromSweep :type Boolean) (SweepResult :type Hit%20Result%20Structure%20%28by%20ref%29))
  (bind _animalcontroller (Variables|Default|GetAnimalController))
  (Utilities|Casting|CastToCapsuleComponent OtherComp)
  (bind _asprey_ai (Utilities|Casting|CastToPreyAI OtherActor))
  (Utilities|IsValid _animalcontroller
    (:Is%20Valid
      (AI|Components|Blackboard|SetValueasObject (Variables|/Script/Animals.AnimalController|GetBlackboardComponent _animalcontroller) (Variables|Default|GetPrey%20Name) _asprey_ai)
      (Variables|Default|SetbChasing true)
      (Variables|/Script/Engine.CharacterMovementComponent|SetMaxWalkSpeed (Variables|Character|GetCharacterMovement) (Variables|Default|GetChasingSpeed))
      (Variables|Default|SetFindPlayerTargetTimer 0.0))))

(event Custom|HunterDeath
  (if (not (Variables|Default|GetbDead))
    (Animation|Montage|MontagePlay (Components|SkeletalMesh|GetAnimInstance (Variables|Character|GetMesh)) "/Game/AI/Hunter/Animations/ANIM_Lion_Death_Montage.ANIM_Lion_Death_Montage" 1.0 "MontageLength" 0.0 true)
    (Variables|Default|SetbDead true)
    (Development|PrintString "Prey is dead")
    (Components|DestroyComponent (Variables|Default|GetSensing%20Sphere))
    (Components|DestroyComponent (Variables|Collision|GetCapsuleComponent))
    (AI|Navigation|StopMovement (Variables|Default|GetAnimalController))))

(fn ConstructionScript)

(fn IsInterestedinPawn
  (params (Pawn :type Pawn%20Object%20Reference%20%28by%20ref%29))
  (return (.bSuccess (Utilities|Casting|CastToFpsPasCharacter Pawn))))